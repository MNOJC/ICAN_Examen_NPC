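; BP_Enemy is an AI enemy character with a floating state widget and a sphere that can trigger the win screen.
; BeginPlay pushes the current EnemyState to the WBP_NPC_StateInfo widget once.
; Tick prints that state for debugging and turns the widget on yaw only to face the player.
; When the player overlaps the sphere while the enemy is in Patrol, it creates and displays WBP_WInScreen.
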(event `self.ReceiveTick`
  (params (DeltaSeconds :type "Float (single-precision)"))
  (`KismetSystemLibrary.PrintString` (`KismetStringLibrary.Concat_StrStr` "CURRENT STATE :" (`|GetEnumeratorNameAsString` (`self.EnemyState`))) true false (struct :`R` 0.3901 :`B` 1.0 :`A` 1.0) 0.0)
  (`self.UpdateWidgetRotation`))

(event `self.ReceiveBeginPlay`
  (bind _aswbp_npc_state_info (cast `/Game/Widget/WBP_NPC_StateInfo` (`WidgetComponent.GetWidget` (`self.Widget`))))
  (bind _output_get (set `self.As WBP NPC State Info` _aswbp_npc_state_info))
  (`/Game/Widget/WBP_NPC_StateInfo.UpdateNPCState` _output_get (`self.EnemyState`)))

(event `self.Sphere.OnComponentBeginOverlap`
  (params (OverlappedComponent :type "PrimitiveComponent Object Reference") (OtherActor :type "Actor Object Reference") (OtherComp :type "PrimitiveComponent Object Reference") (OtherBodyIndex :type Integer) (bFromSweep :type Boolean) (SweepResult :type "HitResult Structure (by ref)"))
  (cast `/Game/FirstPerson/Blueprints/BP_FirstPersonCharacter` OtherActor)
  (switch `/Game/AI/Enums/EEnemyState` (`self.EnemyState`)
    (:`NewEnumerator0`
      (bind _returnvalue (`|CreateWidget` "/Game/Widget/WBP_WInScreen.WBP_WInScreen_C"))
      (`UserWidget.AddToViewport` _returnvalue 0))))

(fn `UpdateWidgetRotation`
  (bind (_returnvalue_roll _returnvalue_pitch _returnvalue_yaw) (`KismetMathLibrary.BreakRotator` (`KismetMathLibrary.FindLookAtRotation` (`self.K2_GetActorLocation`) (`self.K2_GetActorLocation` (`GameplayStatics.GetPlayerCharacter` 0)))))
  (`SceneComponent.K2_SetWorldRotation` (`self.Widget`) (`KismetMathLibrary.MakeRotator` 0.0 0.0 _returnvalue_yaw) false false))

(fn `UserConstructionScript`)